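; Color-coded pressure button that unlocks its target door when a physics pickup of matching color overlaps it.
; The construction script tints the button with a dynamic material instance using the pickup color.
; A matching overlap unlocks the door and plays a timeline that lowers the button mesh.
; Any physics pickup leaving the overlap relocks the door and reverses the timeline, without checking color.
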(event OnComponentBeginOverlap(Overlap)
  (params (OverlappedComponent :type Primitive%20Component%20Object%20Reference) (OtherActor :type Actor%20Object%20Reference) (OtherComp :type Primitive%20Component%20Object%20Reference) (OtherBodyIndex :type Integer) (bFromSweep :type Boolean) (SweepResult :type Hit%20Result%20Structure%20%28by%20ref%29))
  (Development|PrintString "Hello")
  (bind _asphysics_pickup_bp (Utilities|Casting|CastToPhysicsPickup_BP OtherActor))
  (if (== (Variables|/Game/Interactables_AA/PhysicsPickup_BP.PhysicsPickup_BP_C|GetPickup%20Color _asphysics_pickup_bp) (Variables|Default|GetPickup%20Color))
    (Variables|/Game/Interactables_AA/AnimatedInteractables/Door_BP.Door_BP_C|SetisUnlocked (Variables|Default|GetTargetDoor) true)
    (bind _alphatrack (Timeline|Alpha Play)
      (:Update
        (Transformation|SetRelativeLocation (Variables|Default|GetButton) (Math|Vector|MakeVector 0.0 0.0 (Math|Float|Lerp 5.0 1.0 _alphatrack)) false false)))))

(event OnComponentEndOverlap(Overlap)
  (params (OverlappedComponent :type Primitive%20Component%20Object%20Reference) (OtherActor :type Actor%20Object%20Reference) (OtherComp :type Primitive%20Component%20Object%20Reference) (OtherBodyIndex :type Integer))
  (Utilities|Casting|CastToPhysicsPickup_BP OtherActor)
  (Variables|/Game/Interactables_AA/AnimatedInteractables/Door_BP.Door_BP_C|SetisUnlocked (Variables|Default|GetTargetDoor) false)
  (bind _alphatrack (Timeline|Alpha Reverse)
    (:Update
      (Transformation|SetRelativeLocation (Variables|Default|GetButton) (Math|Vector|MakeVector 0.0 0.0 (Math|Float|Lerp 5.0 1.0 _alphatrack)) false false))))

(event EventBeginPlay)

(event Collision|EventActorBeginOverlap
  (params (OtherActor :type Actor%20Object%20Reference)))

(event EventTick
  (params (DeltaSeconds :type Float%20%28single-precision%29)))

(fn ConstructionScript
  (bind _returnvalue (Rendering|Material|CreateDynamicMaterialInstance (Variables|Default|GetButton) 0 "/Game/Interactables_AA/MAT_Color.MAT_Color" "None" :!class /Script/Engine.PrimitiveComponent))
  (bind _output_get (Variables|Default|SetColor%20DMI _returnvalue))
  (Rendering|Material|SetVectorParameterValue _output_get "Color" (Variables|Default|GetPickup%20Color) :!class /Script/Engine.MaterialInstanceDynamic))