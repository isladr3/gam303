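; Interactable door Blueprint that, when unlocked and interacted with, swings open away from or toward the player's side, then closes itself.
; UpdateDoorAngle picks plus or minus 90 degrees from the dot product of the player direction and the door's forward vector.
; A timeline lerps the pivot's yaw, then reverses after a short delay.
; The construction script tints the door through a dynamic material using PickupColor.
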(event Custom|ReverseTimeline
  (bind (_direction _alpha) (Timeline|Timeline Reverse)
    (:Update
      (Transformation|SetRelativeRotation (Variables|Default|GetPivot) (Math|Rotator|MakeRotator 0.0 0.0 (Math|Float|Lerp 0.0 (stale EventINTInteract _returnvalue) _alpha)) false false))
    (:Finished
      (if (Utilities|Enum|Equal(Enum) _direction "Forward")
        (Utilities|FlowControl|Delay 1.0)
        (CallFunction|ReverseTimeline)))))

(event EventINTInteract
  (params (PlayerRef :type Player%20Char%20BP%20Object%20Reference))
  (if (Variables|Default|GetisUnlocked)
    (bind _returnvalue (CallFunction|UpdateDoorAngle PlayerRef))
    (bind (_direction _alpha) (Timeline|Timeline Play)
      (:Update
        (Transformation|SetRelativeRotation (Variables|Default|GetPivot) (Math|Rotator|MakeRotator 0.0 0.0 (Math|Float|Lerp 0.0 _returnvalue _alpha)) false false))
      (:Finished
        (if (Utilities|Enum|Equal(Enum) _direction "Forward")
          (Utilities|FlowControl|Delay 1.0)
          (CallFunction|ReverseTimeline))))))

(fn ConstructionScript
  (bind _returnvalue (Rendering|Material|CreateDynamicMaterialInstance (Variables|Default|GetDoor) 0 "/Game/Interactables_AA/MAT_Color.MAT_Color" "None" :!class /Script/Engine.PrimitiveComponent))
  (bind _output_get (Variables|Default|SetColor%20DMI _returnvalue))
  (Rendering|Material|SetVectorParameterValue _output_get "Color" (Variables|Default|GetPickup%20Color) :!class /Script/Engine.MaterialInstanceDynamic))

(fn UpdateDoorAngle
  (params (self2 :type Actor%20Object%20Reference))
  (return (select (> (Math|Vector|DotProduct (Math|Vector|GetUnitDirection(Vector) (Transformation|GetActorLocation) (Transformation|GetActorLocation self2)) (Transformation|GetActorForwardVector)) 0.0) 9e+01 -9e+01)))