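; AIChar_BP is an enemy AI character that the player can kill by stomping.
; On BeginPlay it makes a single move to a random reachable point nearby, with no repeat afterward.
; Box overlap damages and knocks the player along fixed world -Y; Sphere overlap without upward velocity bounces them, spawns a heart pickup and destroys the enemy.
; Score and health events only update variables, with several empty stub graphs and no health-based death.
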(event OnComponentBeginOverlap(Box)
  (params (OverlappedComponent :type Primitive%20Component%20Object%20Reference) (OtherActor :type Actor%20Object%20Reference) (OtherComp :type Primitive%20Component%20Object%20Reference) (OtherBodyIndex :type Integer) (bFromSweep :type Boolean) (SweepResult :type Hit%20Result%20Structure%20%28by%20ref%29))
  (bind _asplayer_char_bp (Utilities|Casting|CastToPlayerChar_BP OtherActor))
  (Character|LaunchCharacter _asplayer_char_bp "0.000000,-1000.000000,0.000000" false false)
  (Game|Damage|ApplyDamage _asplayer_char_bp 1e+01 0 self))

(event OnComponentBeginOverlap(Sphere)
  (params (OverlappedComponent :type Primitive%20Component%20Object%20Reference) (OtherActor :type Actor%20Object%20Reference) (OtherComp :type Primitive%20Component%20Object%20Reference) (OtherBodyIndex :type Integer) (bFromSweep :type Boolean) (SweepResult :type Hit%20Result%20Structure%20%28by%20ref%29))
  ;[1 1 1 0.5] Stomp Kill
  (bind _asplayer_char_bp (Utilities|Casting|CastToPlayerChar_BP OtherActor))
  (if (<= (.Z (Math|Vector|BreakVector (Transformation|GetVelocity OtherActor))) 0.0)
    (Character|LaunchCharacter _asplayer_char_bp "0.000000,0.000000,800.000000" false true)
    (Game|SpawnActorfromClass "/Game/Interactables_AA/HeartPickup_BP.HeartPickup_BP_C" (Transformation|GetActorTransform) "AlwaysSpawn" "MultiplyWithRoot" 0 0)
    (Actor|DestroyActor)))

(event EventBeginPlay
  (Utilities|FlowControl|Delay 0.2)
  (AI|AIMoveTo self (.RandomLocation (AI|Navigation|GetRandomReachablePointinRadius (Transformation|GetActorLocation) 5e+03 0 0)) 0 5e+01 false
    (:OnSuccess
      _)
    (:OnFail
      _))
  (Utilities|FlowControl|Delay 0.2))

(fn ConstructionScript)

(fn ResetSpeed)

(fn SetHealth
  (params (Min :type Float%20%28double-precision%29) (Max :type Float%20%28double-precision%29)))

(event Custom|AddScore
  (params (Value :type Integer))
  (Variables|Default|SetScore (+ (Variables|Default|GetScore) Value)))

(event Custom|AIHealthBonus
  (params (MaxHealth :type Float%20%28double-precision%29))
  (bind _output_get (Variables|Default|SetMaxHealth MaxHealth))
  (Variables|Default|SetHealth _output_get))

(event Game|Damage|EventAnyDamage
  (params (Damage :type Float%20%28single-precision%29) (DamageType :type Damage%20Type%20Object%20Reference) (InstigatedBy :type Controller%20Object%20Reference) (DamageCauser :type Actor%20Object%20Reference))
  (Variables|Default|SetDamage%20Causer DamageCauser)
  (Variables|Default|SetHealth (- (Variables|Default|GetHealth) Damage)))